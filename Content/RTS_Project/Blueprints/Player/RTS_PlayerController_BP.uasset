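; RTS player controller that handles camera control, unit selection and orders, and HUD setup.
; The camera pawn moves by axis input, screen-edge scrolling and zoom, with gates swapping edge scrolling for rotation while Pan is held.
; Primary input drives the marquee HUD; secondary sends selected units via AI MoveTo with a decal marker, or shows hovered-unit details until a timer detects cursor exit.
; B and V spawn test units at the cursor.
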(event Custom|CheckCursorOverlap
  ;[1 1 1] Check Overlap
  (if (not (== (Variables|HitResult|GetDisplayedHUDActor) (.HitActor (Collision|BreakHitResult (.HitResult (Class|PlayerController|GetHitResultUnderCursorforObjects (Variables|HitResult|GetSelectableObjectsEnum) true))))))
    (Default|CallDestroyUnitHUD)
    (Utilities|Time|InvalidateTimerHandle (stale Input|ActionEvents|InputActionSecondaryAction _returnvalue_3))))

(event Custom|UpdateSelection
  ;[1 1 1] Marquee
  (if (Variables|Marquee|GetIsHoldingInput)
    (Variables|Marquee|SetHoldingTime (+ (Variables|Marquee|GetHoldingTime) (Variables|Default|GetDeltaTime)))
    (Class|RTSMarqueeSelectionIF|OnInputHold(Message) (Variables|References|GetHUDRef))))

(event EventBeginPlay
  ;[1 1 1] Initalisation
  (Utilities|FlowControl|Sequence
    (:then_0
      ;;[1 1 1] Always Place First!
      (Utilities|ReferenceCast))
    (:then_1
      ;;[1 1 1] HUD Init
      (Utilities|SpawnWidgets)
      (UserInterface|Viewport|AddtoViewport (Variables|References|GetHUDGameTimeRef) 1)
      (UserInterface|Viewport|AddtoViewport (Variables|References|GetHUDResourceRef) 0)
      (HUD|SetHUDVisibility "Visible" "HitTestInvisible"))
    (:then_2
      ;;[1 1 1] Cursor Init
      (Input|SetInputModeGameandUI self 0 "DoNotLock" false)
      (Variables|Default|SetbShowMouseCursor true))))

(event EventTick
  (params (DeltaSeconds :type Float%20%28single-precision%29))
  ;[1 1 1] Marquee
  (Variables|Default|SetDeltaTime DeltaSeconds)
  (if (Variables|Marquee|GetIsHoldingInput)
    (CallFunction|UpdateSelection)))

(event Input|ActionEvents|InputActionCameraReset
  (params (Key :type Key%20Structure))
  (bind _camerapawnref (Variables|References|GetCameraPawnRef))
  ;[1 1 1] Reset Zoom & Pan
  (:Pressed
    (Variables|/Script/Engine.SpringArmComponent|SetTargetArmLength (Variables|/Game/RTS_Project/Blueprints/Player/RTS_CameraPawn_BP.RTS_CameraPawn_BP_C|GetSpringArm _camerapawnref) 1.5e+03)
    (Transformation|SetActorRotation _camerapawnref (Math|Rotator|MakeRotator (.Roll (Math|Rotator|BreakRotator (Transformation|GetActorRotation _camerapawnref))) 0.0 0.0))))

(event Input|ActionEvents|InputActionPrimaryAction
  (params (Key :type Key%20Structure))
  (bind _hudref (Variables|References|GetHUDRef))
  ;[1 1 1] Marquee
  (:Pressed
    (if (not (Variables|Marquee|GetIsBuildingModeActive))
      (Class|RTSMarqueeSelectionIF|OnInputStart(Message) _hudref)
      (Variables|Marquee|SetHoldingTime 0.0)
      (Variables|Marquee|SetIsHoldingInput true)))
  (:Released
    (if (not (Variables|Marquee|GetIsBuildingModeActive))
      (Class|RTSMarqueeSelectionIF|OnInputRelease(Message) _hudref (Variables|Marquee|GetHoldingTime))
      (Variables|Marquee|SetIsHoldingInput false))))

(event Input|ActionEvents|InputActionZoomIn
  (params (Key :type Key%20Structure))
  (bind _camerapawnref (Variables|References|GetCameraPawnRef))
  (bind _springarm (Variables|/Game/RTS_Project/Blueprints/Player/RTS_CameraPawn_BP.RTS_CameraPawn_BP_C|GetSpringArm _camerapawnref))
  ;[1 1 1] Zoom In/Out
  (:Pressed
    (Variables|/Script/Engine.SpringArmComponent|SetTargetArmLength _springarm (Math|Float|Clamp(Float) (- (Variables|/Script/Engine.SpringArmComponent|GetTargetArmLength _springarm) (Variables|MovementVariables|GetZoomSpeed)) (Variables|MovementVariables|GetMinZoomLimit) (Variables|MovementVariables|GetMaxZoomLimit)))))

(event Input|ActionEvents|InputActionPan
  (params (Key :type Key%20Structure))
  (bind _camerapawnref (Variables|References|GetCameraPawnRef))
  (bind _camera (Variables|/Game/RTS_Project/Blueprints/Player/RTS_CameraPawn_BP.RTS_CameraPawn_BP_C|GetCamera _camerapawnref))
  (bind _returnvalue (Math|Vector|GetForwardVector _camera))
  (bind _returnvalue_2 (Math|Vector|GetRightVector _camera))
  ;[1 1 1] Edge Scolling
  (:Pressed
    (Utilities|FlowControl|Gate false) ; enters at Close
  )
  (:Released
    (Utilities|FlowControl|Gate false) ; enters at Open
  ))

(event Input|ActionEvents|InputActionPan
  (params (Key :type Key%20Structure))
  (bind _camerapawnref (Variables|References|GetCameraPawnRef))
  (bind _panspeed (Variables|MovementVariables|GetPanSpeed))
  (bind _returnvalue (Transformation|GetActorRotation _camerapawnref))
  (bind (_roll _pitch _yaw) (Math|Rotator|BreakRotator _returnvalue))
  ;[1 1 1] Camera Panning (Rotation)
  (:Pressed
    (Utilities|FlowControl|Gate true) ; enters at Open
  )
  (:Released
    (Utilities|FlowControl|Gate true) ; enters at Close
  ))

(event Input|ActionEvents|InputActionPan
  (params (Key :type Key%20Structure))
  (bind _camerapawnref (Variables|References|GetCameraPawnRef))
  (bind _camera (Variables|/Game/RTS_Project/Blueprints/Player/RTS_CameraPawn_BP.RTS_CameraPawn_BP_C|GetCamera _camerapawnref))
  (bind _returnvalue (Math|Vector|GetForwardVector _camera))
  (bind _returnvalue_2 (Math|Vector|GetRightVector _camera))
  ;[1 1 1] Edge Scolling
  (:Pressed
    (Utilities|FlowControl|Gate false) ; enters at Close
  )
  (:Released
    (Utilities|FlowControl|Gate false) ; enters at Open
  ))

(event Input|ActionEvents|InputActionZoomOut
  (params (Key :type Key%20Structure))
  (bind _camerapawnref (Variables|References|GetCameraPawnRef))
  (bind _springarm (Variables|/Game/RTS_Project/Blueprints/Player/RTS_CameraPawn_BP.RTS_CameraPawn_BP_C|GetSpringArm _camerapawnref))
  ;[1 1 1] Zoom In/Out
  (:Pressed
    (Variables|/Script/Engine.SpringArmComponent|SetTargetArmLength _springarm (Math|Float|Clamp(Float) (+ (Variables|/Script/Engine.SpringArmComponent|GetTargetArmLength _springarm) (Variables|MovementVariables|GetZoomSpeed)) (Variables|MovementVariables|GetMinZoomLimit) (Variables|MovementVariables|GetMaxZoomLimit)))))

(event Input|ActionEvents|InputActionSecondaryAction
  (params (Key :type Key%20Structure))
  (bind (_hitresult _returnvalue) (Game|Player|GetHitResultUnderCursorbyChannel "TraceTypeQuery1" true))
  (bind _selectableobjectsenum (Variables|HitResult|GetSelectableObjectsEnum))
  (bind _hitresult_2 (Class|PlayerController|GetHitResultUnderCursorforObjects _selectableobjectsenum true))
  (bind _hitactor (Collision|BreakHitResult _hitresult_2))
  ;[1 1 1] Unit Details HUD
  (:Pressed
    (if (Variables|HitResult|GetIsUnitSelected)
      (if _returnvalue
        (Variables|UnitControl|SetTargetLocation (.Location (Collision|BreakHitResult _hitresult)))
        (Utilities|FlowControl|Sequence
          (:then_0
            (Utilities|IsValid (Variables|Default|GetPreviousLocationDecal)
              (:Is%20Valid
                (Components|DestroyComponent (Variables|Default|GetPreviousLocationDecal)))
              (:Is%20Not%20Valid
                _))
            (bind _returnvalue_2 (Rendering|Decal|SpawnDecalatLocation "/Game/RTS_Project/Materials/UnitMovement_Mat.UnitMovement_Mat" "32.000000,64.000000,64.000000" (Math|Vector|MakeVector (.x (Variables|UnitControl|GetTargetLocation)) (.y (Variables|UnitControl|GetTargetLocation)) 1.1e+02) "-90.000000,0.000000,0.000000" 0.0))
            (Variables|Default|SetPreviousLocationDecal _returnvalue_2))
          (:then_1
            (for _array_element (Variables|UnitControl|GetSelectedUnits)
              (AI|Navigation|StopMovement (AI|GetAIController _array_element))
              (AI|AIMoveTo (AI|GetAIController _array_element) (Variables|UnitControl|GetTargetLocation) 0 -1.0 "Disable" "Enable" true false
                (:OnMoveFinished
                  (Utilities|IsValid (Variables|Default|GetPreviousLocationDecal)
                    (:Is%20Valid
                      (Components|DestroyComponent (Variables|Default|GetPreviousLocationDecal))))))))))
      (elif (Utilities|IsValid _hitactor)
        (Default|CallDisplayUnitHUD _hitactor false)
        (Variables|HitResult|SetDisplayedHUDActor _hitactor)
        (bind _returnvalue_3 (Utilities|Time|SetTimerbyEvent (delegate Custom|CheckCursorOverlap) 0.5 true))))))

(event Input|AxisEvents|InputAxisMoveForward
  (params (AxisValue :type Float%20%28single-precision%29))
  (bind _camerapawnref (Variables|References|GetCameraPawnRef))
  (bind _camera (Variables|/Game/RTS_Project/Blueprints/Player/RTS_CameraPawn_BP.RTS_CameraPawn_BP_C|GetCamera _camerapawnref))
  (bind _returnvalue (Math|Vector|GetForwardVector _camera))
  ;[1 1 1] Camera Movement
  (if (Variables|MovementVariables|GetMovementEnabled)
    (Transformation|SetActorLocation _camerapawnref (+ (* (Math|Vector|MakeVector (.x _returnvalue) (.y _returnvalue) 0.0) (* (* AxisValue (Variables|MovementVariables|GetMovementSpeedModifier)) 2.0)) (Transformation|GetActorLocation _camerapawnref)) true false)))

(event Input|AxisEvents|InputAxisMoveRight
  (params (AxisValue :type Float%20%28single-precision%29))
  (bind _camerapawnref (Variables|References|GetCameraPawnRef))
  (bind _camera (Variables|/Game/RTS_Project/Blueprints/Player/RTS_CameraPawn_BP.RTS_CameraPawn_BP_C|GetCamera _camerapawnref))
  (bind _returnvalue (Math|Vector|GetRightVector _camera))
  ;[1 1 1] Camera Movement
  (if (Variables|MovementVariables|GetMovementEnabled)
    (Transformation|SetActorLocation _camerapawnref (+ (Transformation|GetActorLocation _camerapawnref) (* (Math|Vector|MakeVector (.x _returnvalue) (.y _returnvalue) 0.0) (* (* AxisValue (Variables|MovementVariables|GetMovementSpeedModifier)) 2.0))) true false)))

(event Input|MouseEvents|MouseY
  (params (AxisValue :type Float%20%28single-precision%29))
  (bind _camerapawnref (Variables|References|GetCameraPawnRef))
  (bind _panspeed (Variables|MovementVariables|GetPanSpeed))
  (bind _returnvalue (Transformation|GetActorRotation _camerapawnref))
  (bind (_roll _pitch _yaw) (Math|Rotator|BreakRotator _returnvalue))
  ;[1 1 1] Camera Panning (Rotation)
  (Utilities|FlowControl|Gate true
    (:Exit
      (Transformation|SetActorRotation _camerapawnref (Math|Rotator|MakeRotator _roll (Math|Float|Clamp(Float) (+ _pitch (* AxisValue _panspeed)) -45.0 45.0) (Math|Float|Clamp(Float) (+ _yaw (* (stale Input|MouseEvents|MouseX AxisValue) _panspeed)) -9e+01 9e+01))))))

(event Input|MouseEvents|MouseX
  (params (AxisValue :type Float%20%28single-precision%29))
  (bind _camerapawnref (Variables|References|GetCameraPawnRef))
  (bind _panspeed (Variables|MovementVariables|GetPanSpeed))
  (bind _returnvalue (Transformation|GetActorRotation _camerapawnref))
  (bind (_roll _pitch _yaw) (Math|Rotator|BreakRotator _returnvalue))
  ;[1 1 1] Camera Panning (Rotation)
  (Utilities|FlowControl|Gate true
    (:Exit
      (Transformation|SetActorRotation _camerapawnref (Math|Rotator|MakeRotator _roll (Math|Float|Clamp(Float) (+ _pitch (* (stale Input|MouseEvents|MouseY AxisValue) _panspeed)) -45.0 45.0) (Math|Float|Clamp(Float) (+ _yaw (* AxisValue _panspeed)) -9e+01 9e+01))))))

(event Input|MouseEvents|MouseX
  (params (AxisValue :type Float%20%28single-precision%29))
  (bind _camerapawnref (Variables|References|GetCameraPawnRef))
  (bind _camera (Variables|/Game/RTS_Project/Blueprints/Player/RTS_CameraPawn_BP.RTS_CameraPawn_BP_C|GetCamera _camerapawnref))
  (bind _returnvalue (Math|Vector|GetForwardVector _camera))
  (bind _returnvalue_2 (Math|Vector|GetRightVector _camera))
  ;[1 1 1] Edge Scolling
  (Utilities|FlowControl|Gate false
    (:Exit
      (bind (_deltaspeedx _deltaspeedy) (Utilities|EdgeScroll))
      (Transformation|SetActorLocation _camerapawnref (+ (+ (* (Math|Vector|MakeVector (.x _returnvalue) (.y _returnvalue) 0.0) _deltaspeedx) (* (Math|Vector|MakeVector (.x _returnvalue_2) (.y _returnvalue_2) 0.0) _deltaspeedy)) (Transformation|GetActorLocation _camerapawnref)) true false))))

(event Input|MouseEvents|MouseY
  (params (AxisValue :type Float%20%28single-precision%29))
  (bind _camerapawnref (Variables|References|GetCameraPawnRef))
  (bind _camera (Variables|/Game/RTS_Project/Blueprints/Player/RTS_CameraPawn_BP.RTS_CameraPawn_BP_C|GetCamera _camerapawnref))
  (bind _returnvalue (Math|Vector|GetForwardVector _camera))
  (bind _returnvalue_2 (Math|Vector|GetRightVector _camera))
  ;[1 1 1] Edge Scolling
  (Utilities|FlowControl|Gate false
    (:Exit
      (Utilities|EdgeScroll) ; enters at MouseY
    )))

(event Input|KeyboardEvents|V
  (params (Key :type Key%20Structure))
  (bind _self self)
  (bind _relativecursorlocationingame (CallFunction|SetCursorWorldPosition _self 1e+04))
  ;[1 1 1] Spawn Text Unit
  (:Pressed
    (Game|SpawnActorfromClass "/Game/RTS_Project/Units/IMP_TIEFighter.IMP_TIEFighter_C" (Math|Transform|MakeTransform (Math|Vector|MakeVector (.x _relativecursorlocationingame) (.y _relativecursorlocationingame) 2e+02)) "Undefined" 0 0)
    (Default|GetAllUnits (Variables|References|GetGameStateRef))))

(event Input|KeyboardEvents|B
  (params (Key :type Key%20Structure))
  (bind _self self)
  (bind _relativecursorlocationingame (CallFunction|SetCursorWorldPosition _self 1e+04))
  ;[1 1 1] Spawn Text Unit
  (:Pressed
    (Game|SpawnActorfromClass "/Game/RTS_Project/Units/IMP_StarDestroyer.IMP_StarDestroyer_C" (Math|Transform|MakeTransform (Math|Vector|MakeVector (.x _relativecursorlocationingame) (.y _relativecursorlocationingame) 2e+02)) "Undefined" 0 0)
    (Default|GetAllUnits (Variables|References|GetGameStateRef))))

(fn ConstructionScript)

(fn SetHUDVisibility
  (params (GameTimeHud :type ESlateVisibility%20Enum :default "Visible") (ResourceHUD :type ESlateVisibility%20Enum :default "Visible"))
  (Widget|SetVisibility (Variables|References|GetHUDGameTimeRef) GameTimeHud)
  (Widget|SetVisibility (Variables|References|GetHUDResourceRef) ResourceHUD))

(fn SetSelectedUnits
  (params (SelectedUnits :type Array%20of%20RTS%20Unit%20Master%20Object%20References))
  (Variables|UnitControl|SetSelectedUnits SelectedUnits)
  (if (>= (Utilities|Array|LastIndex (Variables|UnitControl|GetSelectedUnits)) 0)
    (Variables|HitResult|SetIsUnitSelected true)))