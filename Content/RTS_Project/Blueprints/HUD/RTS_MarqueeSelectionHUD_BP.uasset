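; RTS HUD that draws a drag-selection marquee and selects the units inside it.
; Input start, hold and release events track the rectangle from mouse positions read through the player controller; starting with units already selected only clears them.
; While dragging, DrawHUD rebuilds the selection each frame from RTS_UnitMaster actors in the rectangle, updating their decals.
; Release hands the selected units to the controller.
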(event Custom|DrawMarquee
  (bind _clickedlocation (Variables|Marquee|GetClickedLocation))
  (bind _holdinglocation (Variables|Marquee|GetHoldingLocation))
  (bind _clickedlocation_2 (Variables|Marquee|GetClickedLocation))
  (bind _holdinglocation_2 (Variables|Marquee|GetHoldingLocation))
  (bind (_x _y) (Math|Vector2D|BreakVector2D _holdinglocation))
  (bind (_x_2 _y_2) (Math|Vector2D|BreakVector2D _clickedlocation_2))
  (bind _returnvalue (- _holdinglocation_2 _clickedlocation_2))
  (bind (_x_3 _y_3) (Math|Vector2D|BreakVector2D _clickedlocation))
  (bind (_x_4 _y_4) (Math|Vector2D|BreakVector2D _returnvalue))
  ;[1 1 1] Draw Marquee
  (HUD|DrawRect "(R=1.000000,G=0.417885,B=0.000000,A=1.000000)" _x_3 _y_3 0.0 0.0)
  (HUD|DrawRect "(R=1.000000,G=0.417885,B=0.000000,A=1.000000)" _x _y 0.0 0.0)
  (HUD|DrawRect "(R=1.000000,G=0.417885,B=0.000000,A=0.227000)" _x_2 _y_2 _x_4 _y_4))

(event EventBeginPlay
  ;[1 1 1] BeginPlay
  (bind _asrts_player_controller_bp (Utilities|Casting|CastToRTS_PlayerController_BP (Game|GetPlayerController 0)))
  (Variables|References|SetControllerRef _asrts_player_controller_bp))

(event EventOnInputStart
  (bind _controllerref (Variables|References|GetControllerRef))
  (bind (_locationx _locationy) (Game|Player|GetMousePosition _controllerref))
  ;[1 1 1] Start
  (if (>= (Utilities|Array|LastIndex (Variables|Units|GetSelectedUnits)) 0)
    (for _array_element (Variables|Units|GetSelectedUnits)
      (Default|SetDeselectedDecal _array_element)
      (Variables|/Game/RTS_Project/Units/RTS_UnitMaster.RTS_UnitMaster_C|SetIsSelected _array_element false)
      (Variables|/Game/RTS_Project/Blueprints/Player/RTS_PlayerController_BP.RTS_PlayerController_BP_C|SetIsUnitSelected (Variables|References|GetControllerRef) false))
    (Utilities|Array|Clear (Variables|Units|GetSelectedUnits))
    (else
      (bind _output_get (Variables|Marquee|SetClickedLocation (Math|Vector2D|MakeVector2D _locationx _locationy)))
      (Variables|Marquee|SetHoldingLocation _output_get)
      (Variables|Marquee|SetIsDrawing true))))

(event EventOnInputRelease
  (params (HoldTime :type Float%20%28single-precision%29))
  ;[1 1 1] Release
  (Variables|Marquee|SetIsDrawing false)
  (Default|SetSelectedUnits (Variables|References|GetControllerRef) (Variables|Units|GetSelectedUnits)))

(event EventDrawHUD
  (params (SizeX :type Integer) (SizeY :type Integer))
  (bind _selectedunits (Variables|Units|GetSelectedUnits))
  (bind _selectedunits_2 (Variables|Units|GetSelectedUnits))
  ;[1 1 1] Draw HUD
  (if (Variables|Marquee|GetIsDrawing)
    (Utilities|FlowControl|Sequence
      (:then_0
        (for _array_element _selectedunits_2
          (Default|SetDeselectedDecal _array_element)
          (Utilities|Array|Clear _selectedunits_2)
          (Variables|Units|SetSelectedUnit 0)))
      (:then_1
        (CallFunction|DrawMarquee)
        (bind _output_get (Variables|Units|SetUnitsInSelectionArea (Class|HUD|GetActorsinSelectionRectangle "/Game/RTS_Project/Units/RTS_UnitMaster.RTS_UnitMaster_C" (Variables|Marquee|GetClickedLocation) (Variables|Marquee|GetHoldingLocation) true false)))
        (for _array_element_2 _output_get
          (if (Utilities|ClassIsChildOf (Utilities|GetClass _array_element_2) "/Game/RTS_Project/Units/RTS_UnitMaster.RTS_UnitMaster_C")
            (bind _asrts_unit_master (Utilities|Casting|CastToRTS_UnitMaster _array_element_2))
            (Variables|Units|SetSelectedUnit _asrts_unit_master)
            (Utilities|FlowControl|Sequence
              (:then_0
                (Utilities|Array|AddUnique _selectedunits (Variables|Units|GetSelectedUnit)))
              (:then_1
                (for _array_element_3 _selectedunits
                  (Default|SetSelectedDecal _array_element_3)
                  (Variables|/Game/RTS_Project/Units/RTS_UnitMaster.RTS_UnitMaster_C|SetIsSelected _array_element_3 true))))))))))

(event EventOnInputHold
  (bind _controllerref (Variables|References|GetControllerRef))
  (bind (_locationx _locationy) (Game|Player|GetMousePosition _controllerref))
  ;[1 1 1] Hold
  (Variables|Marquee|SetHoldingLocation (Math|Vector2D|MakeVector2D _locationx _locationy)))

(fn ConstructionScript)