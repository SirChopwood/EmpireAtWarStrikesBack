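; RTS spawn volume that scatters resource actors at random points within its bounds, at BeginPlay and/or on a looping timer.
; SpawnResource box-traces each random point and spawns only on Landscape hits, though totals count requested amounts.
; Timed spawns skip while the HUD game clock is paused and stop at a maximum total.
; Tick recomputes RespawnTime from game-state speed and/or a custom value, but the running timer is never reset.
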(event Custom|SpawnResourcesOnTimer
  (bind _numofresourcesspawn (Variables|ResourceSettings|GetNumOfResourcesSpawn))
  (if (not (Variables|/Game/RTS_Project/Blueprints/Widgets/GameTime_HUD.GameTime_HUD_C|GetIsPaused (Variables|/Game/RTS_Project/Blueprints/Player/RTS_PlayerController_BP.RTS_PlayerController_BP_C|GetHUDGameTimeRef (Variables|References|GetPlayerControllerRef))))
    (if (and (Variables|ResourceSettings|GetIsSpawnOnTimer) (< (Variables|ResourceSettings|GetTotalNumberSpawned) (Variables|ResourceSettings|GetMaxResourcesSpawned)))
      (CallFunction|SpawnResource (Variables|References|GetResourceRef) (- _numofresourcesspawn 1))
      (Variables|ResourceSettings|SetTotalNumberSpawned (+ _numofresourcesspawn (Variables|ResourceSettings|GetTotalNumberSpawned))))))

(event Custom|GetGameSpeed
  (params (GameSpeed :type Float%20%28single-precision%29))
  (Variables|ResourceSettings|SetGameSpeed GameSpeed))

(event EventBeginPlay
  (Utilities|FlowControl|Sequence
    (:then_0
      (Utilities|ReferenceCasts))
    (:then_1
      (EventDispatchers|BindEventtoGameSpeedControl (Variables|References|GetGameStateRef) (EventDispatchers|CreateEvent :!event Custom|GetGameSpeed))
      (bind _gamespeed (Default|GetGameSpeed (Variables|References|GetGameStateRef)))
      (Variables|ResourceSettings|SetGameSpeed _gamespeed)
      (CallFunction|SetRespawnTimer))
    (:then_2
      (if (Variables|ResourceSettings|GetIsSpawnOnBeginPlay)
        (CallFunction|SpawnResource (Variables|References|GetResourceRef) (Variables|ResourceSettings|GetNumOfInitalResources))
        (Variables|ResourceSettings|SetTotalNumberSpawned (+ (Variables|ResourceSettings|GetNumOfInitalResources) (Variables|ResourceSettings|GetTotalNumberSpawned))))
      (if (Variables|ResourceSettings|GetIsSpawnOnTimer)
        (Utilities|Time|SetTimerbyEvent (EventDispatchers|CreateEvent :!event Custom|SpawnResourcesOnTimer) (Variables|ResourceSettings|GetRespawnTime) true)))))

(event EventTick
  (params (DeltaSeconds :type Float%20%28single-precision%29))
  (CallFunction|SetRespawnTimer))

(fn ConstructionScript)

(fn SpawnResource
  (params (Resource :type RTS%20Resource%20Master%20BP%20Class%20Reference) (SpawnAmount :type Integer))
  (bind (_origin _boxextent) (Collision|GetActorBounds false))
  (bind _z (Math|Vector|BreakVector _origin))
  (bind (_x _y) (Math|Vector|BreakVector _boxextent))
  (bind _returnvalue (* _y 2.0))
  (bind _returnvalue_2 (* _x 2.0))
  (bind _returnvalue_3 (- _y _returnvalue))
  (bind _returnvalue_4 (- _x _returnvalue_2))
  (bind _returnvalue_5 (Math|Random|RandomFloatinRange _returnvalue_3 _y))
  (bind _returnvalue_6 (Math|Random|RandomFloatinRange _returnvalue_4 _x))
  (bind _returnvalue_7 (Math|Vector|MakeVector _returnvalue_6 _returnvalue_5 _z))
  (bind _returnvalue_8 (+ _origin _returnvalue_7))
  (LocalVariables|SetResourceRefLocal Resource)
  (bind _output_get (LocalVariables|SetSpawnAmountLocal SpawnAmount))
  (for _index (range 0 _output_get)
    (bind _outhit (Collision|BoxTraceByChannel (+ _returnvalue_8 "0, 0,200.000000") "0, 0, 0" (- _returnvalue_8 (Math|Vector|MakeVector 0.0 0.0 2e+02)) "0, 0, 0" "TraceTypeQuery1" false 0 "None"))
    (if (== (Utilities|GetClass (.HitActor (Collision|BreakHitResult _outhit))) "/Script/Landscape.Landscape")
      (Game|SpawnActorfromClass (LocalVariables|GetResourceRefLocal) (Math|Conversions|ToTransform(Vector) (.Location (Collision|BreakHitResult _outhit))) "Undefined" 0 0))))

(fn SetRespawnTimer
  (bind _userrespawntimer (Variables|ResourceSettings|GetUserRespawnTimer))
  (bind _gamespeed (Variables|ResourceSettings|GetGameSpeed))
  (switch Utilities|FlowControl|Switch|SwitchonRespawnTimer_Enum (Variables|References|GetTimeSettingRef)
    (:NewEnumerator0
      (Variables|ResourceSettings|SetRespawnTime 0.0))
    (:NewEnumerator1
      (Variables|ResourceSettings|SetRespawnTime _gamespeed))
    (:NewEnumerator2
      (Variables|ResourceSettings|SetRespawnTime _userrespawntimer))
    (:NewEnumerator3
      (Variables|ResourceSettings|SetRespawnTime (* _gamespeed _userrespawntimer))))
  (return (Variables|ResourceSettings|GetRespawnTime)))